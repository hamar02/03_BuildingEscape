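; Openable door actor that swings around its yaw axis in response to the OpenDoor OnOpen and OnClose events.
; BeginPlay stores the starting rotation, and a timeline supplies the angle that is combined with it to set the actor's rotation.
; OnOpen plays the timeline and OnClose reverses it.
; InvertOpenAngle selects the swing direction, with a math expression negating the angle when the flag is false.
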(event OnClose(OpenDoor)
  (bind _startrotation (Variables|Default|GetStartRotation))
  (bind _openangle (Timeline|Timeline_DoorAngle Reverse)
    (:Update
      (if (Variables|Default|GetInvertOpenAngle)
        (Transformation|SetActorRotation (Math|Rotator|CombineRotators (Math|Rotator|MakeRotator 0.0 0.0 _openangle) _startrotation))
        (else
          (Transformation|SetActorRotation (Math|Rotator|CombineRotators _startrotation (Math|Rotator|MakeRotator 0.0 0.0 (|Input*Parameter _openangle -1.0)))))))))

(event OnOpen(OpenDoor)
  (bind _startrotation (Variables|Default|GetStartRotation))
  (bind _openangle (Timeline|Timeline_DoorAngle Play)
    (:Update
      (if (Variables|Default|GetInvertOpenAngle)
        (Transformation|SetActorRotation (Math|Rotator|CombineRotators (Math|Rotator|MakeRotator 0.0 0.0 _openangle) _startrotation))
        (else
          (Transformation|SetActorRotation (Math|Rotator|CombineRotators _startrotation (Math|Rotator|MakeRotator 0.0 0.0 (|Input*Parameter _openangle -1.0)))))))))

(event EventBeginPlay
  (Variables|Default|SetStartRotation (Transformation|GetActorRotation)))

(fn ConstructionScript)